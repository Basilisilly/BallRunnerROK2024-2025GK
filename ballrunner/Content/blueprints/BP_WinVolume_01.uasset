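; BP_WinVolume_01 is a level exit volume that leads to level02 once crystals are collected.
; Any overlap with its Box counts remaining BP_Crystal_O2 actors and prints a Polish "not all crystals collected" message if any remain.
; Otherwise it fades the camera out, waits briefly, then opens level02.
; BP_Crystal_O1 actors are also fetched, but their duplicate check branch is disconnected and never runs.
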(event OnComponentBeginOverlap(Box)
  (params (OverlappedComponent :type Primitive%20Component%20Object%20Reference) (OtherActor :type Actor%20Object%20Reference) (OtherComp :type Primitive%20Component%20Object%20Reference) (OtherBodyIndex :type Integer) (bFromSweep :type Boolean) (SweepResult :type Hit%20Result%20Structure%20%28by%20ref%29))
  (bind _outactors (Actor|GetAllActorsOfClass "/Game/blueprints/BP_Crystal_O1.BP_Crystal_O1_C"))
  (bind _outactors_2 (Actor|GetAllActorsOfClass "/Game/blueprints/BP_Crystal_O2.BP_Crystal_O2_C"))
  (if (> (Utilities|Array|Length _outactors_2) 0)
    (Development|PrintString "Nie zebrano wszystkich kryształów")
    (else
      (CameraFades|StartCameraFade :self (Game|GetPlayerCameraManager 0) :ToAlpha 1.0 :Duration 2.0 :bHoldWhenFinished true)
      (Utilities|FlowControl|Delay 2.1)
      (Game|OpenLevel(byName) "level02"))))

(fn ConstructionScript)